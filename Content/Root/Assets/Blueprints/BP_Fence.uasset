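; BP_Fence is a construction-time spline tool that lays out a fence from repeated copies of a chosen mesh.
; The construction script assigns Mesh to an instanced static mesh component, then adds an instance every Spacing units along the spline.
; Each instance takes the spline's local-space transform at that distance, including scale, so it follows the curve.
; The event graph holds only disabled stub events, with no runtime logic.
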(fn `UserConstructionScript`
  (`|ExecutionSequence`
    (:`then_0`
      (`StaticMeshComponent.SetStaticMesh` (`self.InstancedStaticMesh`) (`self.Mesh`)))
    (:`then_1`
      (for _index (range (+ (`KismetMathLibrary.FTrunc` (/ (`SplineComponent.GetSplineLength` (`self.Spline`)) (`self.Spacing`))) 1))
        (`InstancedStaticMeshComponent.AddInstance` (`self.InstancedStaticMesh`) (`SplineComponent.GetTransformAtDistanceAlongSpline` (`self.Spline`) (* _index (`self.Spacing`)) "Local" true))))))