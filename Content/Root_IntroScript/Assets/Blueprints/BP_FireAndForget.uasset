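; BP_FireAndForget is a fire-and-forget missile that flies along a spline toward where the player stood when it began play.
; BeginPlay moves spline point 4 of the missile path to the player character's capsule location, with no later retargeting.
; Each Tick adds Speed to the travelled distance without delta-time scaling and places the Pivot at that spline position and rotation.
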(event `self.ReceiveBeginPlay`
  (`SplineComponent.SetLocationAtSplinePoint` (`self.MIssilePath`) 4 (`SceneComponent.K2_GetComponentLocation` (`Character.CapsuleComponent` (`GameplayStatics.GetPlayerCharacter` 0))) "World" true))

(event `self.ReceiveTick`
  (params (DeltaSeconds :type "Float (single-precision)"))
  (bind (_returnvalue_location _returnvalue_rotation) (`KismetMathLibrary.BreakTransform` (`SplineComponent.GetTransformAtDistanceAlongSpline` (`self.MIssilePath`) (`self.DistanceOnSpline`) "World" false)))
  (set `self.DistanceOnSpline` (+ (`self.Speed`) (`self.DistanceOnSpline`)))
  (`SceneComponent.K2_SetWorldLocationAndRotation` (`self.Pivot`) _returnvalue_location _returnvalue_rotation false false))

(fn `UserConstructionScript`)