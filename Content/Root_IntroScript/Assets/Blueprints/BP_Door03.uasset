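; BP_Door03 is a sliding door that moves open while its Trigger volume is overlapped and back on end overlap.
; The overlap events set an Open flag, and begin overlap also opens a Gate that the opening movement passes through.
; Every Tick eases CurrentPos toward EndPos or StartPos with VInterpTo and applies it as the Door component's relative location.
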(event `self.ReceiveTick`
  (params (DeltaSeconds :type "Float (single-precision)"))
  (if (`self.Open`)
    (`/Engine/EditorBlueprintResources/StandardMacros.Gate` true :!label _label
      (:`Exit`
        (bind _output_get (set `self.CurrentPos` (`KismetMathLibrary.VInterpTo` (`self.CurrentPos`) (`self.EndPos`) (`GameplayStatics.GetWorldDeltaSeconds`) 1.0)))
        (`SceneComponent.K2_SetRelativeLocation` (`self.Door`) _output_get false false)))
    (else
      (bind _output_get_2 (set `self.CurrentPos` (`KismetMathLibrary.VInterpTo` (`self.CurrentPos`) (`self.StartPos`) (`GameplayStatics.GetWorldDeltaSeconds`) 1.0)))
      (`SceneComponent.K2_SetRelativeLocation` (`self.Door`) _output_get_2 false false))))

(event `self.trigger.OnComponentBeginOverlap`
  (params (OverlappedComponent :type "PrimitiveComponent Object Reference") (OtherActor :type "Actor Object Reference") (OtherComp :type "PrimitiveComponent Object Reference") (OtherBodyIndex :type Integer) (bFromSweep :type Boolean) (SweepResult :type "HitResult Structure (by ref)"))
  (set `self.Open` true)
  (goto _label :!via `Open`))

(event `self.trigger.OnComponentEndOverlap`
  (params (OverlappedComponent :type "PrimitiveComponent Object Reference") (OtherActor :type "Actor Object Reference") (OtherComp :type "PrimitiveComponent Object Reference") (OtherBodyIndex :type Integer))
  (set `self.Open` false))

(fn `UserConstructionScript`)