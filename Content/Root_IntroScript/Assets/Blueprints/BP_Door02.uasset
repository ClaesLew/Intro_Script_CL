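; BP_Door02 is a sliding door that rises while something overlaps its Trigger and lowers when the overlap ends.
; Overlap events set the Closed flag and open a gate, and Tick moves the Door's relative location between lower and raised positions using VInterpToConstant.
; Raising uses world delta seconds, while lowering uses a fixed delta, so closing speed depends on frame rate.
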(event `self.ReceiveTick`
  (params (DeltaSeconds :type "Float (single-precision)"))
  (if (`self.closed`)
    (bind _output_get (set `self.CurrentPos` (`KismetMathLibrary.VInterpTo_Constant` (`self.CurrentPos`) (0.0 0.0 150.0) 1.0 1.0)))
    (`SceneComponent.K2_SetRelativeLocation` (`self.Door`) _output_get false false)
    (else
      (`/Engine/EditorBlueprintResources/StandardMacros.Gate` true :!label _label
        (:`Exit`
          (bind _output_get_2 (set `self.CurrentPos` (`KismetMathLibrary.VInterpTo_Constant` (`self.CurrentPos`) (0.0 0.0 400.0) (`GameplayStatics.GetWorldDeltaSeconds`) 100.0)))
          (`SceneComponent.K2_SetRelativeLocation` (`self.Door`) _output_get_2 false false))))))

(event `self.trigger.OnComponentBeginOverlap`
  (params (OverlappedComponent :type "PrimitiveComponent Object Reference") (OtherActor :type "Actor Object Reference") (OtherComp :type "PrimitiveComponent Object Reference") (OtherBodyIndex :type Integer) (bFromSweep :type Boolean) (SweepResult :type "HitResult Structure (by ref)"))
  (set `self.closed` false)
  (goto _label :!via `Open`))

(event `self.trigger.OnComponentEndOverlap`
  (params (OverlappedComponent :type "PrimitiveComponent Object Reference") (OtherActor :type "Actor Object Reference") (OtherComp :type "PrimitiveComponent Object Reference") (OtherBodyIndex :type Integer))
  (set `self.closed` true))

(fn `UserConstructionScript`)