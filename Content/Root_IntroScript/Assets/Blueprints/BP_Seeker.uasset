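; BP_Seeker is a homing missile actor that flies along a spline toward the player and explodes on arrival.
; Each tick it advances a distance by Speed, without delta-time scaling, and places Pivot at that spline transform.
; It then moves the last spline point onto the player's capsule, bending the path to track them.
; At the spline's end it spawns an explosion emitter and destroys itself, applying no damage.
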(event `self.ReceiveBeginPlay`)

(event `self.ReceiveTick`
  (params (DeltaSeconds :type "Float (single-precision)"))
  (bind _missilepath (`self.MIssilePath`))
  (bind _missilepath_2 (`self.MIssilePath`))
  (bind (_returnvalue_location _returnvalue_rotation) (`KismetMathLibrary.BreakTransform` (`SplineComponent.GetTransformAtDistanceAlongSpline` (`self.MIssilePath`) (`self.DistanceOnSpline`) "World" false)))
  (set `self.DistanceOnSpline` (+ (`self.Speed`) (`self.DistanceOnSpline`)))
  (`SceneComponent.K2_SetWorldLocationAndRotation` (`self.Pivot`) _returnvalue_location _returnvalue_rotation false false)
  (`SplineComponent.SetLocationAtSplinePoint` _missilepath (- (`SplineComponent.GetNumberOfSplinePoints` _missilepath) 1) (`SceneComponent.K2_GetComponentLocation` (`Character.CapsuleComponent` (`GameplayStatics.GetPlayerCharacter` 0))) "World" true)
  (if (>= (`self.DistanceOnSpline`) (`SplineComponent.GetSplineLength` (`self.MIssilePath`)))
    (`GameplayStatics.SpawnEmitterAtLocation` "/Game/StarterContent/Particles/P_Explosion.P_Explosion" (`SplineComponent.GetLocationAtSplinePoint` _missilepath_2 (- (`SplineComponent.GetNumberOfSplinePoints` _missilepath_2) 1) "World") (struct) (2.0 2.0 2.0))
    (`self.K2_DestroyActor`)))

(fn `UserConstructionScript`)