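; BP_Door04 is a door that moves open for the player only when they hold the yellow keycard.
; On trigger overlap it checks HasYellowKeycard on Core_GameInstance, then plays the DoorControl timeline or prints a no-keycard debug message.
; The timeline lerps the door's relative location from StartPos to EndPos.
; Leaving the trigger reverses the timeline without a keycard check, and the "HAS KEYCARD" debug print sits on the timeline's Finished output.
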(event `self.Triggger.OnComponentBeginOverlap`
  (params (OverlappedComponent :type "PrimitiveComponent Object Reference") (OtherActor :type "Actor Object Reference") (OtherComp :type "PrimitiveComponent Object Reference") (OtherBodyIndex :type Integer) (bFromSweep :type Boolean) (SweepResult :type "HitResult Structure (by ref)"))
  (cast `/Game/Root_IntroScript/Core/FrameWork/Core_PlayerCharacter` OtherActor)
  (bind _ascore_game_instance (cast `/Game/Root_IntroScript/Core/FrameWork/Core_GameInstance` (`GameplayStatics.GetGameInstance`)))
  (if (`/Game/Root_IntroScript/Core/FrameWork/Core_GameInstance.bHasYellowKeycard` _ascore_game_instance)
    (bind (_direction _alpha) (`Timeline|DoorControl` :!label _label)
      (:`Update`
        (`SceneComponent.K2_SetRelativeLocation` (`self.Door`) (`KismetMathLibrary.VLerp` (`self.StartPos`) (`self.EndPos`) _alpha) false false))
      (:`Finished`
        (`KismetSystemLibrary.PrintString` "HAS KEYCARD")))
    (else
      (`KismetSystemLibrary.PrintString` "NO KEYCARD"))))

(event `self.Triggger.OnComponentEndOverlap`
  (params (OverlappedComponent :type "PrimitiveComponent Object Reference") (OtherActor :type "Actor Object Reference") (OtherComp :type "PrimitiveComponent Object Reference") (OtherBodyIndex :type Integer))
  (cast `/Game/Root_IntroScript/Core/FrameWork/Core_PlayerCharacter` OtherActor)
  (goto _label :!via `Reverse`))

(fn `UserConstructionScript`)